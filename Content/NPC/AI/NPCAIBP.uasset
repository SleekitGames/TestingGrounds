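; AI controller for guard NPCs that runs the GuardBehaviour tree on the PatrolData blackboard from BeginPlay.
; AI perception updates write any sensed actor without the TheWatch tag to the blackboard's enemy key.
; A failed sense update for any such actor clears that key, without checking whether it is the stored enemy.
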(event OnTargetPerceptionUpdated(AIPerception)
  (params (Actor :type Actor%20Object%20Reference) (Stimulus :type AI%20Stimulus%20Structure))
  (bind _blackboardcomp (Variables|Default|GetBlackboardComp))
  (bind _enemykey (Variables|Default|GetEnemyKey))
  (if (not (Actor|ActorHasTag Actor "TheWatch"))
    (if (.bSuccessfullySensed (Utilities|Struct|BreakAIStimulus Stimulus))
      (AI|Components|Blackboard|SetValueasObject _blackboardcomp _enemykey Actor)
      (else
        (AI|Components|Blackboard|ClearValue _blackboardcomp _enemykey)))))

(event EventBeginPlay
  (bind _blackboardcomponent (Class|AIController|UseBlackboard "/Game/NPC/AI/PatrolData.PatrolData"))
  (AI|RunBehaviorTree "/Game/NPC/AI/GuardBehaviour.GuardBehaviour")
  (Variables|Default|SetBlackboardComp _blackboardcomponent))

(fn ConstructionScript)